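; BP_MeleeKamikaze is a melee enemy that blows itself up when it attacks, damaging the player if nearby.
; OnAttack halts movement and sets the attacking animation flag, then waits through a fixed fuse delay before spawning explosion effects and sound.
; Damage scales linearly with player distance, strongest at the center and fading to zero at EffectRadius, then the actor destroys itself.
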(event EventBeginPlay
  (|CallParentFunction) ; This node is disabled and will not be called.\nDrag off pins to build functionality.
)

(event Collision|EventActorBeginOverlap
  (params (OtherActor :type Actor%20Object%20Reference))
  (|CallParentFunction OtherActor) ; This node is disabled and will not be called.\nDrag off pins to build functionality.
)

(event EventTick
  (params (DeltaSeconds :type Float%20%28single-precision%29))
  (|CallParentFunction DeltaSeconds) ; This node is disabled and will not be called.\nDrag off pins to build functionality.
)

(event EventOnAttack
  (bind _returnvalue (Transformation|GetActorLocation))
  (bind _effectradius (Variables|Default|GetEffectRadius))
  ;[1 1 1] Explode OnAttack
  (Class|NavMovementComponent|StopActiveMovement (Variables|Character|GetCharacterMovement))
  (Variables|Default|SetMovementOn false)
  (Variables|/Game/Models/Enemies/BaseEnemyAnimController.BaseEnemyAnimController_C|SetAttackingAnim (Variables|Default|GetMeleeAnimController) true)
  (Utilities|FlowControl|Delay 2.83)
  (Effects|SpawnEmitteratLocation "/Game/PolygonHeist/ParticleFX/FX_Explosion.FX_Explosion" _returnvalue)
  (Audio|PlaySoundatLocation "/Game/Models/Sound/explosion.explosion" _returnvalue "0, 0, 0" 1.0 1.0 0.0 0 0 0)
  ;[1 1 1] Damage player based on distance and destroy self
  (bind _asplayer_character (Utilities|Casting|CastToPlayerCharacter (Game|GetPlayerCharacter 0)))
  (if (<= (Transformation|GetDistanceTo _asplayer_character) _effectradius)
    (Default|GetDamaged _asplayer_character (Math|Float|MapRangeClamped (Transformation|GetDistanceTo _asplayer_character) _effectradius 0.0 0.0 (Variables|Default|GetDamage%20Amount))))
  (Actor|DestroyActor))

(fn ConstructionScript
  (|CallParentFunction))