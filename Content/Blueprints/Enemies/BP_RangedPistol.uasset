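; Ranged enemy that chases a seen player and fires pistol projectiles.
; Pawn sensing drives AI movement to within range, then OnAttack pauses movement and flags the attack animation for a fixed delay.
; A separate OnShoot event spawns the damaging projectile at ShotDirection with muzzle effect and random gunshot sound.
; Death stops movement, flags the death animation and destroys the actor after a delay; construction attaches the pistol to a mesh socket.
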(event OnSeePawn(PawnSensing)
  (params (Pawn :type Pawn%20Object%20Reference))
  ;[1 1 1] Movement logic
  (if (Variables|Default|GetMovement%20On)
    (bind _asplayer_character (Utilities|Casting|CastToPlayerCharacter Pawn))
    (AI|AIMoveTo self "0, 0, 0" _asplayer_character 5e+02 false
      (:OnSuccess
        (CallFunction|OnAttack)))))

(event Custom|OnShoot
  (bind _shotdirection (Variables|Default|GetShotDirection))
  (bind _returnvalue (Transformation|GetWorldLocation _shotdirection))
  (bind _returnvalue_2 (Transformation|GetWorldRotation _shotdirection))
  ;[1 1 1] Shooting behaviour
  (bind _returnvalue_3 (Game|SpawnActorfromClass "/Game/Blueprints/PlayerCharacter/Projectile/Projectile.Projectile_C" (Math|Transform|MakeTransform _returnvalue _returnvalue_2 "1,1,1") "Undefined" self 0))
  (Variables|/Game/Blueprints/PlayerCharacter/Projectile/Projectile.Projectile_C|SetDamage%20Amount _returnvalue_3 (Variables|Default|GetDamage%20Amount))
  (Variables|/Game/Blueprints/PlayerCharacter/Projectile/Projectile.Projectile_C|SetCaster _returnvalue_3 self)
  (Effects|SpawnEmitteratLocation "/Game/PolygonHeist/ParticleFX/FX_Gunshot.FX_Gunshot" _returnvalue _returnvalue_2)
  (Audio|PlaySoundatLocation (Utilities|Array|Get(acopy) (Variables|Default|GetGunshotSounds) (Math|Random|RandomIntegerinRange 0 3)) _returnvalue "0, 0, 0" 0.6 1.0 0.0 0 0 0))

(event EventBeginPlay
  (bind _asbase_enemy_anim_controller (Utilities|Casting|CastToBaseEnemyAnimController (Components|SkeletalMesh|GetAnimInstance (Variables|Character|GetMesh))))
  (Variables|Default|SetAnimController _asbase_enemy_anim_controller))

(event Collision|EventActorBeginOverlap
  (params (OtherActor :type Actor%20Object%20Reference)))

(event EventTick
  (params (DeltaSeconds :type Float%20%28single-precision%29)))

(event EventOnDeath
  ;[1 1 1] OnDeath Behaviour
  (Variables|Default|SetMovement%20On false)
  (Variables|/Game/Models/Enemies/BaseEnemyAnimController.BaseEnemyAnimController_C|SetDeathAnim (Variables|Default|GetAnimController) true)
  (Class|NavMovementComponent|StopActiveMovement (Variables|Character|GetCharacterMovement))
  (Utilities|FlowControl|Delay 3.43)
  (Actor|DestroyActor))

(event EventOnAttack
  (bind _animcontroller (Variables|Default|GetAnimController))
  ;[1 1 1] OnAttack behaviour
  (Variables|/Game/Models/Enemies/BaseEnemyAnimController.BaseEnemyAnimController_C|SetAttackingAnim _animcontroller true)
  (Variables|Default|SetMovement%20On false)
  (Variables|Default|SetIsAttacking true)
  (Utilities|FlowControl|Delay 1.16)
  (Variables|/Game/Models/Enemies/BaseEnemyAnimController.BaseEnemyAnimController_C|SetAttackingAnim _animcontroller false)
  (Variables|Default|SetMovement%20On true)
  (Variables|Default|SetIsAttacking false))

(fn ConstructionScript
  (|CallParentFunction)
  (Transformation|AttachComponentToComponent (Variables|Default|GetPistol) (Variables|Character|GetMesh) "WepSlot" "KeepRelative" "KeepRelative" "KeepRelative" true))