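; Base enemy Blueprint with clamped health, a health bar widget and empty OnDeath and OnAttack events.
; GetDamaged subtracts damage, updates the EnemyHealthWidget display and calls OnDeath when health nears zero, provided the widget cast succeeds.
; Every Tick, the health bar rotates on yaw only to face the player camera, keeping it upright.
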(event Custom|OnDeath)

(event Custom|OnAttack)

(event EventBeginPlay)

(event EventTick
  (params (DeltaSeconds :type Float%20%28single-precision%29))
  (CallFunction|HealthBarLookatCamera))

(event EventGetDamaged
  (params (DamageAmount :type Float%20%28single-precision%29))
  (bind _max_health (Variables|Default|GetMAX_HEALTH))
  ;[1 1 1] Get Damage implementation
  (bind _output_get (Variables|Default|SetHealth (Math|Float|Clamp(Float) (- (Variables|Default|GetHealth) DamageAmount) 0.0 _max_health)))
  (bind _asenemy_health_widget (Utilities|Casting|CastToEnemyHealthWidget (UserInterface|GetWidget (Variables|Default|GetHealthBar))))
  (Default|SetHealthDisplay _asenemy_health_widget _output_get _max_health)
  (if (Math|Float|NearlyEqual(Float) _output_get 0.0 0.1)
    (CallFunction|OnDeath)))

(fn ConstructionScript)

(fn HealthBarLookatCamera
  (bind _healthbar (Variables|Default|GetHealthBar))
  (Transformation|SetWorldRotation _healthbar (Math|Rotator|MakeRotator 0.0 0.0 (.yaw (Math|Rotator|FindLookatRotation (Transformation|GetWorldLocation _healthbar) (Camera|GetCameraLocation (Game|GetPlayerCameraManager 0))))) false false))