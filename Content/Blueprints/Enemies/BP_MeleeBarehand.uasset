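; Blueprint for a barehanded melee enemy that chases the player on sight and punches when it reaches them.
; Pawn sensing drives AI MoveTo, whose success starts an attack that pauses movement and sets flags on the animation controller.
; During the swing, a delayed self-repeating capsule trace at the right-hand socket damages the first player hit and plays a sound.
; Death stops movement, plays the death animation, then destroys the actor.
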(event OnSeePawn(PawnSensing)
  (params (Pawn :type Pawn%20Object%20Reference))
  ;[1 1 1] Movement logic
  (if (Variables|Default|GetMovementOn)
    (bind _asplayer_character (Utilities|Casting|CastToPlayerCharacter Pawn))
    (AI|AIMoveTo self "0, 0, 0" _asplayer_character 5e+01 false
      (:OnSuccess
        (CallFunction|OnAttack)))))

(event Custom|AttackTrace
  (bind _mesh (Variables|Character|GetMesh))
  (bind _returnvalue (Transformation|GetSocketLocation _mesh "Hand_R"))
  ;[1 1 1] Punch Tracing
  (if (Variables|Default|GetIsAttacking)
    (bind (_outhit _returnvalue_2) (Class|KismetSystemLibrary|CapsuleTraceSingleforObjects _returnvalue _returnvalue 15.0 15.0 (Utilities|Array|MakeArray "ObjectTypeQuery3") false 0 "None" true))
    (if _returnvalue_2
      (bind _asplayer_character (Utilities|Casting|CastToPlayerCharacter (.HitActor (Collision|BreakHitResult _outhit))))
      (Default|GetDamaged _asplayer_character (Variables|Default|GetDamage%20Amount))
      (Audio|PlaySoundatLocation (Variables|Default|GetHitSound) (Transformation|GetActorLocation) "0, 0, 0" 1.0 1.0 0.0 0 0 0)
      (else
        (Utilities|FlowControl|Delay 0.01)
        (CallFunction|AttackTrace)))))

(event EventBeginPlay
  (bind _asbase_enemy_anim_controller (Utilities|Casting|CastToBaseEnemyAnimController (Components|SkeletalMesh|GetAnimInstance (Variables|Character|GetMesh))))
  (Variables|Default|SetMeleeAnimController _asbase_enemy_anim_controller))

(event Collision|EventActorBeginOverlap
  (params (OtherActor :type Actor%20Object%20Reference)))

(event EventTick
  (params (DeltaSeconds :type Float%20%28single-precision%29)))

(event EventOnDeath
  ;[1 1 1] OnDeath Behaviour
  (Variables|Default|SetMovementOn false)
  (Variables|/Game/Models/Enemies/BaseEnemyAnimController.BaseEnemyAnimController_C|SetDeathAnim (Variables|Default|GetMeleeAnimController) true)
  (Class|NavMovementComponent|StopActiveMovement (Variables|Character|GetCharacterMovement))
  (Utilities|FlowControl|Delay 3.43)
  (Actor|DestroyActor))

(event EventOnAttack
  (bind _meleeanimcontroller (Variables|Default|GetMeleeAnimController))
  ;[1 1 1] OnAttack behaviour
  (Variables|/Game/Models/Enemies/BaseEnemyAnimController.BaseEnemyAnimController_C|SetAttackingAnim _meleeanimcontroller true)
  (Variables|Default|SetMovementOn false)
  (Variables|Default|SetIsAttacking true)
  (Utilities|FlowControl|Sequence
    (:then_0
      (Utilities|FlowControl|Delay 2.0)
      (Variables|/Game/Models/Enemies/BaseEnemyAnimController.BaseEnemyAnimController_C|SetAttackingAnim _meleeanimcontroller false)
      (Variables|Default|SetMovementOn true)
      (Variables|Default|SetIsAttacking false))
    (:then_1
      (Utilities|FlowControl|Delay 0.4)
      (CallFunction|AttackTrace))))

(fn ConstructionScript
  (|CallParentFunction))